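; Client spawner actor that opens a door and keeps spawning AI clients at its arrow.
; After a start delay, a timeline rotates the door and enters the spawn logic on every update.
; Spawn recursively requests four clients, then resets and waits, but the shared Delay in SpawnClients collapses overlapping requests.
; Pawn class (Poli or Connard) and behavior tree are randomized independently, so they can mismatch.
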(event `SpawnClients`
  (bind _returnvalue (`KismetMathLibrary.RandomInteger` 2))
  (bind _arrow (`self.Arrow`))
  (`KismetSystemLibrary.Delay` 2.0)
  (`AIBlueprintHelperLibrary.SpawnAIFromClass` (select `int` _returnvalue :`0` "/Game/Clients/anims/ClientPoliBP.ClientPoliBP_C" :`1` "/Game/Clients/anims/ClientConnardBP.ClientConnardBP_C" :!type "Pawn Class Reference") (select `int` _returnvalue :`0` "/Game/Clients/anims/ClientBehaviorTree.ClientBehaviorTree" :`1` "/Game/Clients/anims/ClientBehaviorTreeConnard.ClientBehaviorTreeConnard" :!type "BehaviorTree Object Reference") (`SceneComponent.K2_GetComponentLocation` _arrow) (`SceneComponent.K2_GetComponentRotation` _arrow) false null))

(event `Spawn`
  (if (<= (`self.NbOfClients`) 3) :!label _label
    (`self.SpawnClients`)
    (set `self.NbOfClients` (+ (`self.NbOfClients`) 1))
    (`self.Spawn`)
    (else
      (set `self.NbOfClients` 0)
      (`KismetSystemLibrary.Delay` 10.0)
      (`self.Spawn`))))

(event `self.ReceiveBeginPlay`
  (`KismetSystemLibrary.Delay` 5.0)
  (bind (_direction _newtrack_0) (`Timeline|Timeline`)
    (:`Update`
      (`SceneComponent.K2_SetWorldRotation` (`self.door`) (`KismetMathLibrary.MakeRotator` 0.0 0.0 _newtrack_0) false false)
      (goto _label))))

(fn `UserConstructionScript`)