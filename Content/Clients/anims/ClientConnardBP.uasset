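; ClientConnardBP is a client character that reacts to being hit by a baguette.
; Every tick it caches all BP_Bread actors, and on capsule overlap checks whether the other actor is one of them.
; A match turns on mesh physics, adds the bread's EvaluateStars result to the spawner's TotalScore and flags the baguette as received.
; Delayed calls then destroy the bread and, later, the client.
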(event `self.ReceiveTick`
  (params (DeltaSeconds :type "Float (single-precision)"))
  (bind _outactors (`GameplayStatics.GetAllActorsOfClass` "/Game/VRMyAssets/Blueprints/Ingredients/BP_Bread.BP_Bread_C"))
  (set `self.AllBaguettesConnard` _outactors))

(event `self.Capsule.OnComponentBeginOverlap`
  (params (OverlappedComponent :type "PrimitiveComponent Object Reference") (OtherActor :type "Actor Object Reference") (OtherComp :type "PrimitiveComponent Object Reference") (OtherBodyIndex :type Integer) (bFromSweep :type Boolean) (SweepResult :type "HitResult Structure (by ref)"))
  (bind _spawnerref (`self.SpawnerRef`))
  (for _array_element (`self.AllBaguettesConnard`)
    (bind _output_get (set `self.BaguetteConnard` _array_element))
    (if (== _output_get OtherActor)
      (`PrimitiveComponent.SetSimulatePhysics` (`self.Mesh`) true)
      (bind _asbp_bread (cast `/Game/VRMyAssets/Blueprints/Ingredients/BP_Bread` OtherActor))
      (bind _returnvalue (`Ingredient.EvaluateStars` _asbp_bread false))
      (set `/Game/Clients/anims/ClientsSpawnerBP.TotalScore` (+ _returnvalue (`/Game/Clients/anims/ClientsSpawnerBP.TotalScore` _spawnerref)) _spawnerref)
      (set `self.HasBaguetteConnard?` true)
      (`KismetSystemLibrary.Delay` 1.0)
      (`self.K2_DestroyActor` _output_get)
      (`KismetSystemLibrary.Delay` 8.0)
      (`self.K2_DestroyActor`))))

(fn `UserConstructionScript`
  (`parent.UserConstructionScript`))