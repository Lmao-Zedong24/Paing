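; ClientPoliBP is a client actor that takes a baguette on contact and removes itself shortly afterward.
; On BeginPlay it caches all BP_Bread actors, then checks capsule overlaps against that list.
; A match calls the bread's GrabComponent; on success it disables cylinder collision, attaches the socketable component to the RightHand socket keeping world position and rotation, and flags HasBaguette.
; The client destroys itself after a delay.
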(event `self.ReceiveBeginPlay`
  (bind _outactors (`GameplayStatics.GetAllActorsOfClass` "/Game/VRMyAssets/Blueprints/Ingredients/BP_Bread.BP_Bread_C"))
  (set `self.AllBaguettes` _outactors))

(event `self.Capsule.OnComponentBeginOverlap`
  (params (OverlappedComponent :type "PrimitiveComponent Object Reference") (OtherActor :type "Actor Object Reference") (OtherComp :type "PrimitiveComponent Object Reference") (OtherBodyIndex :type Integer) (bFromSweep :type Boolean) (SweepResult :type "HitResult Structure (by ref)"))
  (bind _refsocket (`self.RefSocket`))
  (for _array_element (`self.AllBaguettes`)
    (bind _output_get (set `self.BaguetteRef` _array_element))
    (if (== OtherActor _output_get)
      (bind _isheld (`/Game/VRTemplate/Blueprints/GrabComponent.TryGrab` (`/Game/VRMyAssets/Blueprints/Ingredients/BP_Bread.GrabComponent` _output_get) _refsocket))
      (if _isheld
        (`PrimitiveComponent.SetCollisionEnabled` (`/Game/VRMyAssets/Blueprints/Ingredients/BP_Bread.Cylinder` _output_get) "NoCollision")
        (`SceneComponent.K2_AttachToComponent` (`/Game/VRMyAssets/Blueprints/Ingredients/BP_Bread.BP_SocketableComponent` _output_get) _refsocket "RightHand" "KeepWorld" "KeepWorld" "KeepRelative" true)
        (set `self.HasBaguette?` true)
        (`KismetSystemLibrary.Delay` 8.0)
        (`self.K2_DestroyActor`)))))

(fn `UserConstructionScript`)