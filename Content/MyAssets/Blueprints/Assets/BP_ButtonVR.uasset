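; BP_ButtonVR is a physics-driven push button for VR.
; When the Button component overlaps PressedCollider, ButtonActivated zeroes its velocity, sets ButtonDown, fires the OnButtonPressed dispatcher and prints a debug string.
; Ending that overlap clears ButtonDown.
; CanMove sets a vertical position target on the PhysicsConstraint, but nothing in these graphs calls it.
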(event `self.PressedCollider.OnComponentBeginOverlap`
  (params (OverlappedComponent :type "PrimitiveComponent Object Reference") (OtherActor :type "Actor Object Reference") (OtherComp :type "PrimitiveComponent Object Reference") (OtherBodyIndex :type Integer) (bFromSweep :type Boolean) (SweepResult :type "HitResult Structure (by ref)"))
  (if (== OtherComp (`self.Button`))
    (`self.ButtonActivated`)))

(event `self.PressedCollider.OnComponentEndOverlap`
  (params (OverlappedComponent :type "PrimitiveComponent Object Reference") (OtherActor :type "Actor Object Reference") (OtherComp :type "PrimitiveComponent Object Reference") (OtherBodyIndex :type Integer))
  (if (== OtherComp (`self.Button`))
    (set `self.ButtonDown` false)))

(fn `ButtonActivated`
  (`PrimitiveComponent.SetPhysicsLinearVelocity` (`self.Button`) (0.0 0.0 0.0) false "None")
  (set `self.ButtonDown` true)
  (`self.OnButtonPressed`)
  (`KismetSystemLibrary.PrintString` "ButtonActivated"))

(fn `CanMove`
  (`PhysicsConstraintComponent.SetLinearPositionTarget` (`self.PhysicsConstraint`) (`KismetMathLibrary.MakeVector` 0.0 0.0 20.0)))

(fn `UserConstructionScript`)