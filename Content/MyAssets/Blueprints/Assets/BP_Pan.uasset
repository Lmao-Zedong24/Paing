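; BP_Pan is a grabbable pan that can sit in a socket and also carries three fixed sockets of its own.
; The construction script assigns a separate box collider to each fixed socket component.
; When the grab component reports a grab, the socketable component lets go if it holds a valid socket reference.
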(event `self.GrabComponent.OnGrabbed`
  (bind _bp_socketablecomponent (`self.BP_SocketableComponent`))
  ;[1 1 1] Release Socket On Grabed
  (`/Engine/EditorBlueprintResources/StandardMacros.IsValid` (`/Game/MyAssets/Blueprints/Sockets/BP_SocketableComponent.SocketRef` _bp_socketablecomponent)
    (:`Is Valid`
      (`/Game/MyAssets/Blueprints/Sockets/BP_SocketableComponent.TryLetGo` _bp_socketablecomponent))))

(fn `UserConstructionScript`
  (set `/Game/MyAssets/Blueprints/Sockets/BP_FixedSocketComponent.Collider` (`self.Box1`) (`self.BP_FixedSocketComponent1`))
  (set `/Game/MyAssets/Blueprints/Sockets/BP_FixedSocketComponent.Collider` (`self.Box2`) (`self.BP_FixedSocketComponent2`))
  (set `/Game/MyAssets/Blueprints/Sockets/BP_FixedSocketComponent.Collider` (`self.Box3`) (`self.BP_FixedSocketComponent3`)))