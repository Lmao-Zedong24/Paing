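; BP_Bread is a VR bread prop that can be grabbed and placed into sockets.
; It pairs a GrabComponent with a BPSocketableComponent, binding a socket-attempt condition at BeginPlay that refuses socketing while the bread is held.
; When grabbed, it notifies the socketable component to release from its current socket if one is valid.
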(event `self.ReceiveBeginPlay`
  ;[1 1 1] Prevent Socket When Grabed
  (add `/Game/VRMyAssets/Blueprints/Sockets/BP_SocketableComponent.ConditionsTrySocket` (`self.BP_SocketableComponent`) (delegate `CustomEvent`)))

(event `CustomEvent`
  ;[1 1 1] Prevent Socket When Grabed
  (if (`/Game/VRTemplate/Blueprints/GrabComponent.bIsHeld` (`self.GrabComponent`))
    (`/Game/VRMyAssets/Blueprints/Sockets/BP_SocketableComponent.CanNotSocket` (`self.BP_SocketableComponent`))))

(event `self.GrabComponent.OnGrabbed`
  ;[1 1 1] Release Socket On Grabed
  (`/Engine/EditorBlueprintResources/StandardMacros.IsValid` (`/Game/VRMyAssets/Blueprints/Sockets/BP_SocketableComponent.SocketRef` (`self.BP_SocketableComponent`))
    (:`Is Valid`
      (`/Game/VRMyAssets/Blueprints/Sockets/BP_SocketableComponent.GotGrabbed` (`self.BP_SocketableComponent`)))))

(fn `UserConstructionScript`)