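; BP_Rack is a rack actor that detects when pans are placed in it and signals when it is full.
; A box trigger counts overlapping BP_Pan mesh components up and down, calling the OnRackFull dispatcher once when the count reaches three, latched by HasTp.
; The construction script pairs Socket1, Socket3 and Socket5 with their collider boxes, while the assignments for Socket2 and Socket4 are disconnected.
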(event `self.ReceiveBeginPlay`)

(event `self.Box.OnComponentBeginOverlap`
  (params (OverlappedComponent :type "PrimitiveComponent Object Reference") (OtherActor :type "Actor Object Reference") (OtherComp :type "PrimitiveComponent Object Reference") (OtherBodyIndex :type Integer) (bFromSweep :type Boolean) (SweepResult :type "HitResult Structure (by ref)"))
  (cast `MeshComponent` OtherComp)
  (cast `/Game/VRMyAssets/Blueprints/Assets/BP_Pan` OtherActor)
  (bind _result (`/Engine/EditorBlueprintResources/StandardMacros.IncrementInt` (`self.NumTrays`))
    (:`  `
      (`/Engine/EditorBlueprintResources/StandardMacros.CompareInt` _result 3
        (:`>`
          _)
        (:`==`
          _))
      (if (not (`self.HasTp`))
        (`self.OnRackFull`)
        (set `self.HasTp` true)))))

(event `self.Box.OnComponentEndOverlap`
  (params (OverlappedComponent :type "PrimitiveComponent Object Reference") (OtherActor :type "Actor Object Reference") (OtherComp :type "PrimitiveComponent Object Reference") (OtherBodyIndex :type Integer))
  (cast `MeshComponent` OtherComp)
  (cast `/Game/VRMyAssets/Blueprints/Assets/BP_Pan` OtherActor)
  (`/Engine/EditorBlueprintResources/StandardMacros.DecrementInt` (`self.NumTrays`)))

(fn `UserConstructionScript`
  (set `/Game/VRMyAssets/Blueprints/Sockets/BP_FixedSocketComponent.Collider` (`self.Box2`) (`self.Socket1`))
  (set `/Game/VRMyAssets/Blueprints/Sockets/BP_FixedSocketComponent.Collider` (`self.Box6`) (`self.Socket5`))
  (set `/Game/VRMyAssets/Blueprints/Sockets/BP_FixedSocketComponent.Collider` (`self.Box4`) (`self.Socket3`)))