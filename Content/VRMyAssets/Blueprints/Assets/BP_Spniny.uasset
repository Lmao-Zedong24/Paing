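; BP_Spniny is a grabbable physics door that stays still unless held and reports when it is closed.
; Tick zeroes the Cube's linear and angular velocity while GrabComponent is not held, and a drop clears it immediately and again after a short timer.
; When the Cube overlaps BoxCenter, it sets IsClosed, forces a drop and calls OnDoorClosed; leaving resets the flag.
; BoxPlus and BoxMinus overlap handlers are empty.
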(event `self.ReceiveTick`
  (params (DeltaSeconds :type "Float (single-precision)"))
  (if (not (`/Game/VRTemplate/Blueprints/GrabComponent.bIsHeld` (`self.GrabComponent`)))
    (`self.ClearVelocity`)))

(event `self.GrabComponent.OnDropped`
  (`self.ClearVelocity`)
  (`KismetSystemLibrary.K2_SetTimer` null "ClearVelocity" 0.2))

(event `self.BoxCenter.OnComponentBeginOverlap`
  (params (OverlappedComponent :type "PrimitiveComponent Object Reference") (OtherActor :type "Actor Object Reference") (OtherComp :type "PrimitiveComponent Object Reference") (OtherBodyIndex :type Integer) (bFromSweep :type Boolean) (SweepResult :type "HitResult Structure (by ref)"))
  (if (== OtherComp (`self.Cube`))
    (set `self.IsClosed` true)
    (`/Game/VRTemplate/Blueprints/GrabComponent.TryDrop` (`self.GrabComponent`))
    (`self.OnDoorClosed`)
    (`KismetSystemLibrary.PrintString` "Door Closed")))

(event `self.BoxCenter.OnComponentEndOverlap`
  (params (OverlappedComponent :type "PrimitiveComponent Object Reference") (OtherActor :type "Actor Object Reference") (OtherComp :type "PrimitiveComponent Object Reference") (OtherBodyIndex :type Integer))
  (if (== OtherComp (`self.Cube`))
    (set `self.IsClosed` false)))

(event `self.BoxPlus.OnComponentBeginOverlap`
  (params (OverlappedComponent :type "PrimitiveComponent Object Reference") (OtherActor :type "Actor Object Reference") (OtherComp :type "PrimitiveComponent Object Reference") (OtherBodyIndex :type Integer) (bFromSweep :type Boolean) (SweepResult :type "HitResult Structure (by ref)")))

(event `self.BoxMinus.OnComponentBeginOverlap`
  (params (OverlappedComponent :type "PrimitiveComponent Object Reference") (OtherActor :type "Actor Object Reference") (OtherComp :type "PrimitiveComponent Object Reference") (OtherBodyIndex :type Integer) (bFromSweep :type Boolean) (SweepResult :type "HitResult Structure (by ref)")))

(fn `ClearVelocity`
  (`PrimitiveComponent.SetAllPhysicsAngularVelocityInDegrees` (`self.Cube`) (`KismetMathLibrary.MakeVector` 0.0) false)
  (`PrimitiveComponent.SetAllPhysicsLinearVelocity` (`self.Cube`) (0.0 0.0 0.0) false)
  (return))

(fn `GetAngularVelocity`
  (returns (AngulatVelocity :type "Vector Structure") (`Relative Rotation` :type "Rotator Structure"))
  (locals (NewLocalVar :type "Vector Structure" :default (0.0 0.0 0.0)))
  (bind _cube (`self.Cube`))
  (return (`PrimitiveComponent.GetPhysicsAngularVelocityInDegrees` _cube "None") (`SceneComponent.RelativeRotation` _cube)))

(fn `UserConstructionScript`)