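; Grabbable VR flour bag that pours flour into containers when tilted about 60 degrees or more from upright.
; Tick checks the up vector and accumulates time while tilted, periodically pouring an amount scaled by that time and the flour rate.
; PourFlour traces from the opening's lowest point and adds the amount to any hit actor's Container component.
; ResetFlourBag drops the bag, teleports it to its spawn transform and clears physics velocities.
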(event `self.ReceiveBeginPlay`
  (set `self.SpawnTrans` (`self.GetTransform`)))

(event `self.ReceiveTick`
  (params (DeltaSeconds :type "Float (single-precision)"))
  (`/Engine/EditorBlueprintResources/StandardMacros.CompareFloat` (`KismetMathLibrary.Dot_VectorVector` (`self.GetActorUpVector`) (0.0 0.0 1.0)) 0.5
    (:`==`
      _)
    (:`<`
      _))
  (`self.Timer` DeltaSeconds
    (:`TimerHit`
      (`self.PourFlour` (* (`self.AcumulatedTime_s`) (`self.Flour_L/s`)))
      (set `self.AcumulatedTime_s` 0.0))))

(fn `PourFlour`
  (params (Amount :type "Float (double-precision)"))
  (bind _returnvalue (`ContainerOpening.GetLowestPointOnOpening` (`self.Opening`)))
  (bind _returnvalue_2 (`Ingredient.PourLiquidTrace` self (`self.Liquid`) (`local.Amount`) _returnvalue))
  (bind (_bblockinghit _binitialoverlap _time _distance _location _impactpoint _normal _impactnormal _physmat _hitactor) (`GameplayStatics.BreakHitResult` _returnvalue_2))
  (if _bblockinghit
    (bind _returnvalue_3 (`self.GetComponentByClass` _hitactor "/Script/Paing2.Container"))
    (`/Engine/EditorBlueprintResources/StandardMacros.IsValid` _returnvalue_3
      (:`Is Valid`
        (bind _returnvalue_4 (`Container.TryAddAmount` _returnvalue_3 (`self.Liquid`) (`local.Amount`)))
        (if _returnvalue_4
          _)))))

(fn `ResetFlourBag`
  (`/Game/VRTemplate/Blueprints/GrabComponent.TryDrop` (`self.GrabComponent`))
  (`self.K2_SetActorTransform` (`self.SpawnTrans`) false true)
  (`PrimitiveComponent.SetPhysicsLinearVelocity` (`self.RootMesh`) (0.0 0.0 0.0) false "None")
  (`PrimitiveComponent.SetPhysicsAngularVelocityInRadians` (`self.RootMesh`) (0.0 0.0 0.0) false "None"))

(fn `UserConstructionScript`)