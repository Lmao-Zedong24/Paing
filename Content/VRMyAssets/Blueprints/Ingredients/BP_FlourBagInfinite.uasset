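; Flour bag ingredient that endlessly pours flour from its cube's position, with no supply to deplete.
; Tick feeds a Timer macro that accumulates delta time and, once past the interval, pours an amount scaled by the flour rate and elapsed time.
; PourFlour reuses the liquid pour trace and tries to add the ingredient to the Container component of any actor it hits.
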(event `self.ReceiveTick`
  (params (DeltaSeconds :type "Float (single-precision)"))
  (`self.Timer` DeltaSeconds
    (:`TimerHit`
      (`self.PourFlour` (* (`self.AcumulatedTime_s`) (`self.Flour_L/s`)))
      (set `self.AcumulatedTime_s` 0.0))))

(fn `PourFlour`
  (params (Amount :type "Float (double-precision)"))
  (bind _returnvalue (`Ingredient.PourLiquidTrace` self (`self.Liquid`) (`local.Amount`) (`SceneComponent.K2_GetComponentLocation` (`self.Cube`))))
  (bind (_bblockinghit _binitialoverlap _time _distance _location _impactpoint _normal _impactnormal _physmat _hitactor) (`GameplayStatics.BreakHitResult` _returnvalue))
  (if _bblockinghit
    (bind _returnvalue_2 (`self.GetComponentByClass` _hitactor "/Script/Paing2.Container"))
    (`/Engine/EditorBlueprintResources/StandardMacros.IsValid` _returnvalue_2
      (:`Is Valid`
        (bind _returnvalue_3 (`Container.TryAddAmount` _returnvalue_2 (`self.Liquid`) (`local.Amount`)))
        (if _returnvalue_3
          _)))))

(fn `UserConstructionScript`)