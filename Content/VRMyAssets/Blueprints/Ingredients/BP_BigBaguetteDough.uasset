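; BP_BigBaguetteDough is a baguette dough ingredient actor that can be squished by shrinking its scale over time.
; StartSquish sets the Squish flag, and Tick then subtracts SquishSpeedScalePerS, scaled by delta time, from the actor's scale.
; Squishing stops once the Z scale is no longer above SquishScaleZ.
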(event `self.ReceiveBeginPlay`)

(event `self.ReceiveTick`
  (params (DeltaSeconds :type "Float (single-precision)"))
  (if (`self.Squish`)
    (`self.SetActorScale3D` (- (`self.GetActorScale3D` self) (* (`self.SquishSpeed_ScalePerS`) DeltaSeconds)))
    (set `self.Squish` (> (.z (`self.GetActorScale3D` self)) (`self.SquishScaleZ`)))))

(fn `StartSquish`
  (set `self.Squish` true))

(fn `UserConstructionScript`)