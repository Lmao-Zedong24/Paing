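; Spawner actor that replenishes a configurable actor class whenever the last spawned one leaves its spawn zone.
; BeginPlay binds the zone's overlap delegates and optionally spawns at the SpawnPoint transform, printing red warnings if the zone or class is unset.
; End overlap spawns a replacement when a static mesh component of the tracked Spawned actor exits.
; The begin-overlap handler is empty.
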(event `self.ReceiveBeginPlay`
  (bind _spawnzone (`self.SpawnZone`)
    (:`then`
      (add `PrimitiveComponent.OnComponentBeginOverlap` _spawnzone (`|CreateDelegate` :!event `OnBegin`))
      (add `PrimitiveComponent.OnComponentEndOverlap` _spawnzone (`|CreateDelegate` :!event `OnEnd`))
      (if (`self.SpawnOnBegin`)
        (`self.Spawn`)))
    (:`else`
      (`KismetSystemLibrary.PrintString` "Set Spawn Zone in spawner" true true (struct :`R` 1.0 :`A` 1.0) 15.0))))

(fn `OnBegin`
  (params (OverlappedComponent :type "PrimitiveComponent Object Reference") (OtherActor :type "Actor Object Reference") (OtherComp :type "PrimitiveComponent Object Reference") (OtherBodyIndex :type Integer) (bFromSweep :type Boolean) (SweepResult :type "HitResult Structure (by ref)"))
  (return))

(fn `OnEnd`
  (params (OverlappedComponent :type "PrimitiveComponent Object Reference") (OtherActor :type "Actor Object Reference") (OtherComp :type "PrimitiveComponent Object Reference") (OtherBodyIndex :type Integer))
  (cast `StaticMeshComponent` OtherComp)
  (if (== OtherActor (`self.Spawned`))
    (`self.Spawn`)))

(fn `Spawn`
  (bind _actortospawn (`self.ActorToSpawn`)
    (:`then`
      (bind _returnvalue (`|SpawnActorFromClass` _actortospawn (`SceneComponent.K2_GetComponentToWorld` (`self.SpawnPoint`)) "AlwaysSpawn" "MultiplyWithRoot" null null))
      (set `self.Spawned` _returnvalue))
    (:`else`
      (`KismetSystemLibrary.PrintString` "Set Actor to spawn in spawner" true true (struct :`R` 1.0 :`A` 1.0) 15.0))))

(fn `UserConstructionScript`)