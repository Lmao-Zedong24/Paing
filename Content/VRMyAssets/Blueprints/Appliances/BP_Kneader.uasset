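; VR kneader appliance that crafts dough from ingredients placed in its sphere trigger, using the big-dough recipe.
; Overlaps add or remove container ingredients, and reaching one ingredient resets the spin count of Spiny, an editor-linked actor.
; It mirrors Spiny's rotation, sets its spin target and binds its target-hit event alongside a spawned VR button's press.
; Crafting checks CanCraft, waits on a timer, and CraftFinished crafts with a sound.
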(event `self.ReceiveBeginPlay`
  (bind _returnvalue (`|SpawnActorFromClass` "/Game/VRMyAssets/Blueprints/Assets/BP_ButtonVR.BP_ButtonVR_C" (`SceneComponent.K2_GetComponentToWorld` (`self.ButtonPos`)) "AlwaysSpawn" "MultiplyWithRoot" null null))
  (`self.K2_AttachToActor` _returnvalue null "None" "KeepRelative" "KeepRelative" "KeepRelative" true)
  (bind _output_get (set `self.Button` _returnvalue))
  (add `/Game/VRMyAssets/Blueprints/Assets/BP_ButtonVR.OnButtonPressed` _output_get (`|CreateDelegate` :!event `TryCraftDough`))
  (bind _spiny (`self.Spiny`)
    (:`then`
      (add `/Game/VRMyAssets/Blueprints/Assets/BP_Spniny.OnHitTarget` _spiny (`|CreateDelegate` :!event `TryCraftDough`))
      (set `/Game/VRMyAssets/Blueprints/Assets/BP_Spniny.SpinTarget_deg` (* (`self.NumSpinsForCraft`) 360.0) _spiny)
      (set `self.m_recipe` "/Game/VRMyAssets/DataAssets/Recipes/DA_BigDough.DA_BigDough"))
    (:`else`
      (`KismetSystemLibrary.PrintString` "Spiny not linked to Kneader in editor " true true (struct :`R` 1.0 :`A` 1.0) 15.0))))

(event `self.ReceiveTick`
  (params (DeltaSeconds :type "Float (single-precision)"))
  (bind (_angulatvelocity _relative_rotation) (`/Game/VRMyAssets/Blueprints/Assets/BP_Spniny.GetAngularVelocity` (`self.Spiny`)))
  (if (!= _angulatvelocity (0.0 0.0 0.0))
    (`SceneComponent.K2_SetRelativeRotation` (`self.Spiner`) _relative_rotation false false)))

(event `self.Sphere.OnComponentBeginOverlap`
  (params (OverlappedComponent :type "PrimitiveComponent Object Reference") (OtherActor :type "Actor Object Reference") (OtherComp :type "PrimitiveComponent Object Reference") (OtherBodyIndex :type Integer) (bFromSweep :type Boolean) (SweepResult :type "HitResult Structure (by ref)"))
  (bind _container (`self.Container`))
  (bind _asingredient (cast `Ingredient` OtherActor))
  (`Container.TryAddIngredient` _container _asingredient)
  (`KismetSystemLibrary.PrintString` "Ingredient Added")
  (`self.PrintIngredients`)
  (bind _returnvalue (`Container.GetIngredientNames` _container))
  (`/Engine/EditorBlueprintResources/StandardMacros.CompareInt` (`BlueprintSetLibrary.Set_Length` _returnvalue) 1
    (:`==`
      (`/Game/VRMyAssets/Blueprints/Assets/BP_Spniny.ResetAccumulated` (`self.Spiny`)))))

(event `self.Sphere.OnComponentEndOverlap`
  (params (OverlappedComponent :type "PrimitiveComponent Object Reference") (OtherActor :type "Actor Object Reference") (OtherComp :type "PrimitiveComponent Object Reference") (OtherBodyIndex :type Integer))
  (bind _asingredient (cast `Ingredient` OtherActor))
  (`Container.TryRemoveIngredient` (`self.Container`) _asingredient)
  (`KismetSystemLibrary.PrintString` "Ingredient Removed"))

(fn `CraftFinished`
  (`self.Craft`)
  (`GameplayStatics.PlaySoundAtLocation` null (`self.K2_GetActorLocation`) (struct) 1.0 1.0 0.0 null null null null))

(fn `PrintIngredients`
  (bind _returnvalue (`Container.GetIngredientNames` (`self.Container`)))
  (bind _result (`BlueprintSetLibrary.Set_ToArray` _returnvalue))
  (for _array_element _result
    (`KismetSystemLibrary.PrintString` (`KismetStringLibrary.Conv_NameToString` _array_element)))
  (return))

(fn `TryCraftDough`
  (bind _returnvalue (`self.CanCraft` self))
  (if _returnvalue
    (`KismetSystemLibrary.K2_SetTimerDelegate` (`|CreateDelegate` :!event `CraftFinished`) (`/Game/VRMyAssets/DataAssets/CrafterInfo/BP_CrafterInfo.CraftDelay_s` (`self.CrafterInfo`)))))

(fn `UserConstructionScript`)