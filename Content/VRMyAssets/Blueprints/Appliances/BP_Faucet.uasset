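; BP_Faucet is a VR faucet that pours a limited supply of water into containers beneath it.
; On BeginPlay it spawns and attaches a BP_ButtonVR whose press toggles the open state.
; While open with water remaining, Tick accumulates time and periodically pours flow rate times elapsed time, using a liquid trace to find a Container component.
; Each pour depletes the supply, hit or not, and rescales the water-level visualizer's Z.
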(event `self.ReceiveBeginPlay`
  ;[1 1 1] Setup Button
  (bind _returnvalue (`|SpawnActorFromClass` "/Game/VRMyAssets/Blueprints/Assets/BP_ButtonVR.BP_ButtonVR_C" (`SceneComponent.K2_GetComponentToWorld` (`self.ButtonPos`)) "AlwaysSpawn" "MultiplyWithRoot" null null))
  (`self.K2_AttachToActor` _returnvalue null "None" "KeepRelative" "KeepRelative" "KeepRelative" true)
  (bind _output_get (set `self.Button` _returnvalue))
  (add `/Game/VRMyAssets/Blueprints/Assets/BP_ButtonVR.OnButtonPressed` _output_get (delegate `OnButtonPressed_Event`)))

(event `OnButtonPressed_Event`
  ;[1 1 1] Setup Button
  (set `self.isFaucetOpen` (not (`self.isFaucetOpen`))))

(event `self.ReceiveTick`
  (params (DeltaSeconds :type "Float (single-precision)"))
  (`self.InterpretFaucetState`
    (:`FaucetOpen`
      (`self.FaucetOpen` DeltaSeconds))))

(fn `FaucetOpen`
  (params (deltaTime_s :type "Float (double-precision)"))
  (bind _faucetinfo (`self.FaucetInfo`))
  (bind _returnvalue (* (`self.AcumulatedTime_s`) (`/Game/VRMyAssets/DataAssets/FaucetInfo/BP_FaucetInfo.waterSpeed_LperS` (`self.FaucetInfo`))))
  (`self.Timer` deltaTime_s
    (:`TimerHit`
      (`self.PourWater` _returnvalue)
      (set `/Game/VRMyAssets/DataAssets/FaucetInfo/BP_FaucetInfo.currentWaterAmount_L` (- (`/Game/VRMyAssets/DataAssets/FaucetInfo/BP_FaucetInfo.currentWaterAmount_L` (`self.FaucetInfo`)) _returnvalue) (`self.FaucetInfo`))
      (set `self.AcumulatedTime_s` 0.0)
      (`SceneComponent.SetRelativeScale3D` (`self.WaterAmountVisualizer`) (`KismetMathLibrary.MakeVector` (.x (`SceneComponent.RelativeScale3D` (`self.WaterAmountVisualizer`))) (.y (`SceneComponent.RelativeScale3D` (`self.WaterAmountVisualizer`))) (/ (`/Game/VRMyAssets/DataAssets/FaucetInfo/BP_FaucetInfo.currentWaterAmount_L` _faucetinfo) (`/Game/VRMyAssets/DataAssets/FaucetInfo/BP_FaucetInfo.maxWaterAmount_L` _faucetinfo)))))))

(fn `PourWater`
  (params (Amount :type "Float (double-precision)"))
  (bind _returnvalue (`Ingredient.PourLiquidTrace` self (`self.waterIngredient`) (`local.Amount`) (`SceneComponent.K2_GetComponentLocation` (`self.WaterSpawnPoint`))))
  (bind (_bblockinghit _binitialoverlap _time _distance _location _impactpoint _normal _impactnormal _physmat _hitactor) (`GameplayStatics.BreakHitResult` _returnvalue))
  (if _bblockinghit
    (bind _returnvalue_2 (`self.GetComponentByClass` _hitactor "/Script/Paing2.Container"))
    (`/Engine/EditorBlueprintResources/StandardMacros.IsValid` _returnvalue_2
      (:`Is Valid`
        (bind _returnvalue_3 (`Container.TryAddAmount` _returnvalue_2 (`self.waterIngredient`) (`local.Amount`)))
        (if _returnvalue_3
          _))
      (:`Is Not Valid`
        (if true
          _)))))

(fn `UserConstructionScript`)