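; BP_Divider is a VR dough divider appliance that crafts from ingredients placed in its box.
; Overlaps add or remove ingredients in its Container, and big baguette dough starts squishing on entry.
; It spawns an attached VR button and binds events to its press and to the closing of an editor-linked door.
; TryDivideDough checks craftability, switches the door lock state, then crafts after a timer and switches it back.
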(event `self.ReceiveBeginPlay`
  ;[1 1 1] Setup Button
  (bind _returnvalue (`|SpawnActorFromClass` "/Game/VRMyAssets/Blueprints/Assets/BP_ButtonVR.BP_ButtonVR_C" (`SceneComponent.K2_GetComponentToWorld` (`self.ButtonPos`)) "AlwaysSpawn" "MultiplyWithRoot" null null))
  (`self.K2_AttachToActor` _returnvalue null "None" "KeepRelative" "KeepRelative" "KeepRelative" true)
  (bind _output_get (set `self.Button` _returnvalue))
  (add `/Game/VRMyAssets/Blueprints/Assets/BP_ButtonVR.OnButtonPressed` _output_get (`|CreateDelegate` :!event `TryDivideDough`))
  (bind _doorup (`self.DoorUp`)
    (:`then`
      (add `/Game/VRMyAssets/Blueprints/Assets/BP_Door.OnDoorClosed` _doorup (`|CreateDelegate` :!event `TryDivideDough`)))
    (:`else`
      (`KismetSystemLibrary.PrintString` "Link Door to Divider in editor" true true (struct :`R` 1.0 :`A` 1.0) 15.0))))

(event `self.ReceiveTick`
  (params (DeltaSeconds :type "Float (single-precision)")))

(event `self.Box.OnComponentBeginOverlap`
  (params (OverlappedComponent :type "PrimitiveComponent Object Reference") (OtherActor :type "Actor Object Reference") (OtherComp :type "PrimitiveComponent Object Reference") (OtherBodyIndex :type Integer) (bFromSweep :type Boolean) (SweepResult :type "HitResult Structure (by ref)"))
  (bind _asingredient (cast `Ingredient` OtherActor))
  (bind _asbp_big_baguette_dough (cast `/Game/VRMyAssets/Blueprints/Ingredients/BP_BigBaguetteDough` _asingredient)
    (:`then`
      (`/Game/VRMyAssets/Blueprints/Ingredients/BP_BigBaguetteDough.StartSquish` _asbp_big_baguette_dough))
    (:`CastFailed`
      _))
  (`Container.TryAddIngredient` (`self.Container`) _asingredient)
  (`KismetSystemLibrary.PrintString` "Ingredient Added"))

(event `self.Box.OnComponentEndOverlap`
  (params (OverlappedComponent :type "PrimitiveComponent Object Reference") (OtherActor :type "Actor Object Reference") (OtherComp :type "PrimitiveComponent Object Reference") (OtherBodyIndex :type Integer))
  (bind _asingredient (cast `Ingredient` OtherActor))
  (`Container.TryRemoveIngredient` (`self.Container`) _asingredient)
  (`KismetSystemLibrary.PrintString` "Ingredient Removed"))

(fn `EndCraft`
  (`self.Craft` self)
  (`/Game/VRMyAssets/Blueprints/Assets/BP_Door.DoorLockState` (`self.DoorUp`) true))

(fn `TryDivideDough`
  (bind _returnvalue (`self.CanCraft` self))
  (if _returnvalue
    (`/Game/VRMyAssets/Blueprints/Assets/BP_Door.DoorLockState` (`self.DoorUp`) false)
    (`KismetSystemLibrary.K2_SetTimer` null "EndCraft" (`self.TimeBeforeCraft_s`))
    (return)))

(fn `UserConstructionScript`)